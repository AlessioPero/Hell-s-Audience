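; BP_SuperHit is a power-up Blueprint in the player power-up system, currently a stub for a super hit with four strength tiers.
; On BeginPlay it finds the top-level PlayerInGameHUD widget and caches the first result.
; Weak, Medium, Strong and SuperStrong events each only print their tier name, and none of them uses the cached widget yet.
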(event Custom|Weak
  (Development|PrintString "WEAK"))

(event Custom|Super%20Strong
  (Development|PrintString "SUPER STRONG"))

(event Custom|Medium
  (Development|PrintString "MEDIUM"))

(event Custom|Strong
  (Development|PrintString "STRONG"))

(event EventBeginPlay
  (bind _foundwidgets (Widget|GetAllWidgetsOfClass "/Game/GameUI/PlayerInGameHUD.PlayerInGameHUD_C" true))
  (Variables|Default|SetWidget (Utilities|Array|Get(acopy) _foundwidgets)))