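; Player power-up Blueprint that spends Hype on timed damage, health and speed boosts.
; DMGUP, HPUP and SPEEDUP each fetch the player character, check and deduct Hype stored on the PlayerInGameHUD widget, double a stat, then halve it after a delay.
; SPEEDUP writes the doubled MaxCustomMovementSpeed only to its own variable, never back to the character's movement component.
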(event Custom|SPEED%20UP
  (bind _asbp_first_person_character (Utilities|Casting|CastToBP_FirstPersonCharacter (Game|GetPlayerCharacter 0)))
  (Variables|Default|SetAs%20BP%20First%20Person%20Character _asbp_first_person_character)
  (bind _foundwidgets (Widget|GetAllWidgetsOfClass "/Game/GameUI/PlayerInGameHUD.PlayerInGameHUD_C" true))
  (if (>= (Variables|/Game/GameUI/PlayerInGameHUD.PlayerInGameHUD_C|GetHype (Utilities|Array|Get(acopy) _foundwidgets)) 20000)
    (Variables|/Game/GameUI/PlayerInGameHUD.PlayerInGameHUD_C|SetHype (Utilities|Array|Get(acopy) _foundwidgets) (- (Variables|/Game/GameUI/PlayerInGameHUD.PlayerInGameHUD_C|GetHype (Utilities|Array|Get(acopy) _foundwidgets)) 20000))
    (Variables|Default|SetMax%20Custom%20Movement%20Speed (* (Variables|/Script/Engine.CharacterMovementComponent|GetMaxCustomMovementSpeed (Variables|/Script/Engine.Character|GetCharacterMovement (Variables|Default|GetAs%20BP%20First%20Person%20Character))) 2.0))
    (Utilities|FlowControl|Delay 1e+01)
    (Variables|Default|SetMax%20Custom%20Movement%20Speed (/ (Variables|Default|GetMax%20Custom%20Movement%20Speed) 2.0))))

(event Custom|DMG%20UP
  (bind _asbp_first_person_character (Utilities|Casting|CastToBP_FirstPersonCharacter (Game|GetPlayerCharacter 0)))
  (Variables|Default|SetAs%20BP%20First%20Person%20Character _asbp_first_person_character)
  (bind _foundwidgets (Widget|GetAllWidgetsOfClass "/Game/GameUI/PlayerInGameHUD.PlayerInGameHUD_C" true))
  (if (>= (Variables|/Game/GameUI/PlayerInGameHUD.PlayerInGameHUD_C|GetHype (Utilities|Array|Get(acopy) _foundwidgets)) 20000)
    (Variables|/Game/Player/FirstPerson/Blueprints/BP_FirstPersonCharacter.BP_FirstPersonCharacter_C|SetDamage (Variables|Default|GetAs%20BP%20First%20Person%20Character) (* (Variables|/Game/Player/FirstPerson/Blueprints/BP_FirstPersonCharacter.BP_FirstPersonCharacter_C|GetDamage (Variables|Default|GetAs%20BP%20First%20Person%20Character)) 2.0))
    (Variables|/Game/GameUI/PlayerInGameHUD.PlayerInGameHUD_C|SetHype (Utilities|Array|Get(acopy) _foundwidgets) (- (Variables|/Game/GameUI/PlayerInGameHUD.PlayerInGameHUD_C|GetHype (Utilities|Array|Get(acopy) _foundwidgets)) 20000))
    (Utilities|FlowControl|Delay 3.0)
    (Variables|/Game/Player/FirstPerson/Blueprints/BP_FirstPersonCharacter.BP_FirstPersonCharacter_C|SetDamage (Variables|Default|GetAs%20BP%20First%20Person%20Character) (/ (Variables|/Game/Player/FirstPerson/Blueprints/BP_FirstPersonCharacter.BP_FirstPersonCharacter_C|GetDamage (Variables|Default|GetAs%20BP%20First%20Person%20Character)) 2.0))))

(event Custom|HP%20UP
  (bind _asbp_first_person_character (Utilities|Casting|CastToBP_FirstPersonCharacter (Game|GetPlayerCharacter 0)))
  (Variables|Default|SetAs%20BP%20First%20Person%20Character _asbp_first_person_character)
  (bind _foundwidgets (Widget|GetAllWidgetsOfClass "/Game/GameUI/PlayerInGameHUD.PlayerInGameHUD_C" true))
  (if (>= (Variables|/Game/GameUI/PlayerInGameHUD.PlayerInGameHUD_C|GetHype (Utilities|Array|Get(acopy) _foundwidgets)) 10000)
    (Variables|/Game/GameUI/PlayerInGameHUD.PlayerInGameHUD_C|SetHype (Utilities|Array|Get(acopy) _foundwidgets) (- (Variables|/Game/GameUI/PlayerInGameHUD.PlayerInGameHUD_C|GetHype (Utilities|Array|Get(acopy) _foundwidgets)) 10000))
    (Variables|/Game/Player/FirstPerson/Blueprints/BP_FirstPersonCharacter.BP_FirstPersonCharacter_C|SetMaxHealth (Variables|Default|GetAs%20BP%20First%20Person%20Character) (* (Variables|/Game/Player/FirstPerson/Blueprints/BP_FirstPersonCharacter.BP_FirstPersonCharacter_C|GetMaxHealth (Variables|Default|GetAs%20BP%20First%20Person%20Character)) 2.0))
    (Variables|/Game/Player/FirstPerson/Blueprints/BP_FirstPersonCharacter.BP_FirstPersonCharacter_C|SetHealth (Variables|Default|GetAs%20BP%20First%20Person%20Character) (* (Variables|/Game/Player/FirstPerson/Blueprints/BP_FirstPersonCharacter.BP_FirstPersonCharacter_C|GetHealth (Variables|Default|GetAs%20BP%20First%20Person%20Character)) 2.0))
    (Utilities|FlowControl|Delay 1e+01)
    (Variables|/Game/Player/FirstPerson/Blueprints/BP_FirstPersonCharacter.BP_FirstPersonCharacter_C|SetMaxHealth (Variables|Default|GetAs%20BP%20First%20Person%20Character) (/ (Variables|/Game/Player/FirstPerson/Blueprints/BP_FirstPersonCharacter.BP_FirstPersonCharacter_C|GetMaxHealth (Variables|Default|GetAs%20BP%20First%20Person%20Character)) 2.0))
    (Variables|/Game/Player/FirstPerson/Blueprints/BP_FirstPersonCharacter.BP_FirstPersonCharacter_C|SetHealth (Variables|Default|GetAs%20BP%20First%20Person%20Character) (/ (Variables|/Game/Player/FirstPerson/Blueprints/BP_FirstPersonCharacter.BP_FirstPersonCharacter_C|GetHealth (Variables|Default|GetAs%20BP%20First%20Person%20Character)) 2.0))))