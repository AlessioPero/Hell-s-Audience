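; Enemy spawner actor that holds a queue of enemy classes and spawns them at its own transform.
; A looping timer started at BeginPlay tries to spawn the queue's first entry, removing it once spawned.
; Newly queued enemies also trigger an immediate spawn when the sphere overlaps no base enemy.
; Each spawned enemy's destroyed delegate is bound, and OnEnemyDefeated relays defeats to the first-person GameMode.
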(event Custom|Try_To_Spawn
  (CallFunction|SpawnEnemy))

(event Custom|On%20Enemy%20Defeated
  (bind _asbp_first_person_game_mode (Utilities|Casting|CastToBP_FirstPersonGameMode (Game|GetGameMode)))
  (Default|OnEnemyDefeated _asbp_first_person_game_mode))

(event EventBeginPlay
  (Utilities|Time|SetTimerbyEvent (delegate Custom|Try_To_Spawn) 2.0 true))

(fn ConstructionScript)

(fn SpawnEnemy
  (if (Utilities|Array|IsValidIndex (Variables|Default|GetEnemyQueue))
    (bind _returnvalue (Game|SpawnActorfromClass (Utilities|Array|Get(acopy) (Variables|Default|GetEnemyQueue)) (Transformation|GetActorTransform) "AdjustIfPossibleButAlwaysSpawn" "MultiplyWithRoot" 0 0))
    (EventDispatchers|BindEventtoOnDestroyed _returnvalue (EventDispatchers|CreateEvent :!event OnENemyDefeated))
    (Utilities|Array|RemoveIndex (Variables|Default|GetEnemyQueue))
    (return true)
    (else
      (return false))))

(fn AddEnemytoQueue
  (params (EnemyType :type BP%20Base%20Enemy%20Class%20Reference%20%28by%20ref%29))
  (Utilities|Array|Add (Variables|Default|GetEnemyQueue) EnemyType)
  (if (not (Utilities|Array|IsValidIndex (Collision|GetOverlappingActors (Variables|Default|GetSphere) "/Game/Enemies/Mannequin/Base/BP_BaseEnemy.BP_BaseEnemy_C" :!class /Script/Engine.PrimitiveComponent)))
    (CallFunction|SpawnEnemy)))