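; BP_Drop handles enemy death drops, giving a one-in-two chance to spawn a health pickup.
; OnDeathDrop takes the transform of the first actor tagged "Enemy", which is not necessarily the one that died, and spawns the health drop there regardless of collision.
; The pickup is stored in HealthItem and set to its own current location, and BeginPlay and Tick are unused.
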(event Custom|OnDeathDrop
  (bind _outactors (Actor|GetAllActorswithTag "Enemy"))
  (switch int (Math|Random|RandomInteger 2)
    (:0
      (bind _returnvalue (Game|SpawnActorfromClass "/Game/Enemies/Drop/BP_Health_Drop.BP_Health_Drop_C" (Math|Transform|MakeTransform (Math|Vector|MakeVector (.X (Math|Vector|BreakVector (.location (Transformation|GetActorTransform (Utilities|Array|Get(acopy) _outactors))))) (.Y (Math|Vector|BreakVector (.location (Transformation|GetActorTransform (Utilities|Array|Get(acopy) _outactors))))) (.Z (Math|Vector|BreakVector (.location (Transformation|GetActorTransform (Utilities|Array|Get(acopy) _outactors)))))) (.rotation (Transformation|GetActorTransform (Utilities|Array|Get(acopy) _outactors))) (.scale (Transformation|GetActorTransform (Utilities|Array|Get(acopy) _outactors)))) "AlwaysSpawn" "MultiplyWithRoot" 0 0))
      (Variables|Default|SetHealthItem _returnvalue)
      (Variables|Default|SetHealthItemLoc (Transformation|GetActorLocation _returnvalue))
      (Transformation|SetActorLocation (Variables|Default|GetHealthItem) (Variables|Default|GetHealthItemLoc) false false))))

(event EventBeginPlay)

(event EventTick
  (params (DeltaSeconds :type Float%20%28single-precision%29)))