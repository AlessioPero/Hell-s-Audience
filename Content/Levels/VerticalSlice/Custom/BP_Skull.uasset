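; BP_Skull is a level actor that keeps turning to face player 0's pawn and carries two point lights.
; From BeginPlay, FacePlayer re-calls itself every 0.1 seconds, interpolating pitch and yaw toward the pawn using frame delta time rather than the loop interval.
; The construction script uses the Sphere component's scaled radius as both attenuation radius and intensity for both lights, so resizing it scales the glow.
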(event Custom|Face%20Player
  (bind _returnvalue (Game|Player|GetPlayerPawn 0))
  (bind _returnvalue_2 (Transformation|GetActorLocation))
  (bind _returnvalue_3 (Transformation|GetActorRotation))
  (bind _returnvalue_4 (Utilities|Time|GetWorldDeltaSeconds))
  (bind _returnvalue_5 (Transformation|GetActorLocation _returnvalue))
  (bind _returnvalue_6 (Math|Rotator|FindLookatRotation _returnvalue_2 _returnvalue_5))
  (bind _returnvalue_7 (Math|Interpolation|RInterpTo _returnvalue_3 _returnvalue_6 _returnvalue_4 2e+01))
  (Transformation|SetActorRotation (Math|Rotator|MakeRotator 0.0 (.pitch _returnvalue_7) (.yaw _returnvalue_7)))
  (Utilities|FlowControl|Delay 0.1)
  (CallFunction|FacePlayer))

(event EventBeginPlay
  (CallFunction|FacePlayer))

(fn ConstructionScript
  (bind _sphere (Variables|Default|GetSphere))
  (bind _returnvalue (Components|Sphere|GetScaledSphereRadius _sphere))
  (Rendering|Lighting|SetAttenuationRadius (Variables|Default|GetPointLight1) _returnvalue)
  (Rendering|Components|Light|SetIntensity (Variables|Default|GetPointLight2) _returnvalue))