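; BP_LaunchPad is a jump pad that launches the first-person player character upward on overlap, then goes on cooldown.
; An active launch plays a sound, swaps the mesh to the offline material and starts a timer.
; The timer's refresh event reactivates the pad, plays a charge sound and restores the ready material after a short delay.
; Every player overlap decreases hype through the in-game HUD widget, even during cooldown.
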(event Custom|RefreshJumpPad
  (Variables|Default|SetIsActive true)
  (Audio|PlaySoundatLocation "/Game/Player/Sounds/Interactables/Jump/A_Jump_Charge.A_Jump_Charge" (Transformation|GetActorLocation) "0, 0, 0" 1.0 1.0 0.0 0 0 0 0)
  (Utilities|FlowControl|Delay 0.5)
  (Rendering|Material|SetMaterial (Variables|Default|GetSM_LaunchPad) 0 "/Game/JumpingPad/Materials/LauncPadReady.LauncPadReady"))

(event Collision|EventActorBeginOverlap
  (params (OtherActor :type Actor%20Object%20Reference))
  (bind _asbp_first_person_character (Utilities|Casting|CastToBP_FirstPersonCharacter OtherActor))
  (bind _foundwidgets (Widget|GetAllWidgetsOfClass "/Game/GameUI/PlayerInGameHUD.PlayerInGameHUD_C" true))
  (Default|DecreaseHype (Utilities|Array|Get(acopy) _foundwidgets) 25000)
  (if (Variables|Default|GetIsActive)
    (Rendering|Material|SetMaterial (Variables|Default|GetSM_LaunchPad) 0 "/Game/JumpingPad/Materials/LauncPadReady.LauncPadReady")
    (Character|LaunchCharacter _asbp_first_person_character (Math|Vector|MakeVector 0.0 0.0 (Variables|Default|GetHigh)) false false)
    (Audio|PlaySoundatLocation "/Game/Player/Sounds/Interactables/Jump/A_Jump.A_Jump" (Transformation|GetActorLocation) "0, 0, 0" 1.0 1.0 0.0 0 0 0 0)
    (Variables|Default|SetIsActive false)
    (Rendering|Material|SetMaterial (Variables|Default|GetSM_LaunchPad) 0 "/Game/JumpingPad/Materials/LauncPadOffline.LauncPadOffline")
    (Utilities|Time|SetTimerbyEvent (delegate Custom|RefreshJumpPad) (Variables|Default|GetCoolDown))
    (else
      (Character|LaunchCharacter _asbp_first_person_character "0, 0, 0" false false))))

(fn ConstructionScript)